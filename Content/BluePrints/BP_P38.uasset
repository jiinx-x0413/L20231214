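; BP_P38 is a player-controlled P-38 aircraft that rolls, pitches, boosts and fires rockets.
; On BeginPlay it registers its Right and Left components with BPPropell, while Roll and Pitch axes apply frame-rate-independent local rotation.
; Fire spawns a BP_Rocket at LaunchPoint.
; Holding Left Shift, bound as a raw key, toggles boost on BPMovement and attaches a spark emitter at BackFirePoint until release.
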(event EventBeginPlay
  (bind _bp_propell (Variables|Default|GetBP_Propell))
  (bind _scenecomponents (Variables|/Game/BluePrints/BP_Propell.BP_Propell_C|GetSceneComponents _bp_propell))
  (Utilities|Array|Add _scenecomponents (Variables|Default|GetRight))
  (Utilities|Array|Add _scenecomponents (Variables|Default|GetLeft)))

(event Input|ActionEvents|InputActionFire
  (params (Key :type Key%20Structure :default "None"))
  (bind _self self)
  ;[0 0 0] Fire
  (:Pressed
    (Game|SpawnActorfromClass "/Game/BluePrints/BP_Rocket.BP_Rocket_C" (Transformation|GetWorldTransform (Variables|Default|GetLaunchPoint)) "Undefined" "MultiplyWithRoot" _self _self)))

(event Input|AxisEvents|InputAxisRoll
  (params (AxisValue :type Float%20%28single-precision%29))
  ;[0 0 0] Input
  (Transformation|AddActorLocalRotation (Math|Rotator|MakeRotator (* AxisValue (Utilities|Time|GetWorldDeltaSeconds) (Variables|Default|GetBodyRotateSpeed)) 0.0 0.0) false false))

(event Input|AxisEvents|InputAxisPitch
  (params (AxisValue :type Float%20%28single-precision%29))
  ;[0 0 0] Input
  (Transformation|AddActorLocalRotation (Math|Rotator|MakeRotator 0.0 (* AxisValue (Utilities|Time|GetWorldDeltaSeconds) (Variables|Default|GetBodyRotateSpeed)) 0.0) false false))

(event Input|KeyboardEvents|LeftShift
  (params (Key :type Key%20Structure :default "None"))
  (bind _bp_movement (Variables|Default|GetBP_Movement))
  ;[0 0 0] Boost
  (:Pressed
    (Default|StartBoost _bp_movement)
    (bind _returnvalue (Effects|SpawnEmitterAttached "/Game/StarterContent/Particles/P_Sparks.P_Sparks" (Variables|Default|GetBackFirePoint) "None" "0, 0, 0" "0, 0, 0" "0.500000,0.540000,0.500000" "SnapToTargetIncludingScale"))
    (Variables|Default|SetEmitterObject _returnvalue))
  (:Released
    (Default|StopBoost _bp_movement)
    (Components|DestroyComponent (Variables|Default|GetEmitterObject))))

(fn ConstructionScript)