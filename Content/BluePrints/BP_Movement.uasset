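; BP_Movement is a component that constantly moves its owning actor forward, with a switchable speed boost.
; Each tick it offsets the owner along its forward vector by MoveSpeed scaled by world delta time, without sweeping for collisions.
; StartBoost and StopBoost switch MoveSpeed between BoostSpeed and DefaultSpeed, and BeginPlay calls StopBoost to begin at the default.
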(event Custom|StartBoost
  (Variables|Speed|SetMoveSpeed (Variables|Default|GetBoostSpeed)))

(event Custom|StopBoost
  (Variables|Speed|SetMoveSpeed (Variables|Default|GetDefaultSpeed)))

(event EventTick
  (params (DeltaSeconds :type Float%20%28single-precision%29))
  (bind _returnvalue (Components|GetOwner))
  (Transformation|AddActorWorldOffset _returnvalue (* (Utilities|Time|GetWorldDeltaSeconds) (Variables|Speed|GetMoveSpeed) (Transformation|GetActorForwardVector _returnvalue))))

(event EventBeginPlay
  (CallFunction|StopBoost))